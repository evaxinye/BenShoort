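; Behavior tree task that picks the next patrol waypoint for an AI-controlled ThirdPersonCharacter.
; On execute it copies the pawn's PatrolPoints array, then writes the point at the blackboard Index into the WayPoint key.
; It advances Index with a modulo of the array length so the patrol loops, then finishes successfully.
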(event `self.ReceiveExecuteAI`
  (params (OwnerController :type "AIController Object Reference") (ControlledPawn :type "Pawn Object Reference"))
  ;[1 1 1] 带有controller 的 ai 会调用这个函数
  ;[1 1 1] 初始化PatrolPoints
  (`self.InitialPatrolPoints` ControlledPawn)
  ;[1 1 1] 根据index , 设置下一个巡逻地点
  (`self.SetNextPoint`)
  ;[1 1 1] 让index在长度范围内循环
  (`self.CycleIndex`)
  (`self.FinishExecute` true))

(fn `CycleIndex`
  (`BTFunctionLibrary.SetBlackboardValueAsInt` (`self.Index`) (mod (+ (`BTFunctionLibrary.GetBlackboardValueAsInt` (`self.Index`)) 1) (`KismetArrayLibrary.Array_Length` (`self.PatrolPoints`)))))

(fn `InitialPatrolPoints`
  (params (Object :type "Object Object Reference"))
  (bind _asthird_person_character (cast `/Game/Core/AI/ThirdPersonCharacter` Object))
  (set `self.PatrolPoints` (`/Game/Core/AI/ThirdPersonCharacter.PatrolPoints` _asthird_person_character)))

(fn `SetNextPoint`
  (`BTFunctionLibrary.SetBlackboardValueAsObject` (`self.WayPoint`) (`|GetArrayItem` (`self.PatrolPoints`) (`BTFunctionLibrary.GetBlackboardValueAsInt` (`self.Index`)))))